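; Player-style ball pawn exposing Rotate, Move and Ability functions, with movement input following the mesh's forward vector after yaw rotation.
; Ability switches on CurrentAbility: Levitate disables gravity and jumps the pawn upward, while TimeSlow lowers time dilation on every A_Crusher.
; Each ability clears CurrentAbility and starts a timer.
; The matching end functions undo the effect and restore that ability if none has replaced it.
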(event `self.ReceiveTick`
  (params (DeltaSeconds :type "Float (single-precision)")))

(fn `Ability`
  (switch `/Game/E_Ability` (`self.CurrentAbility`)
    (:`NewEnumerator1`
      ;[0.776 0.401 0.008084 0.5] LEVITATE
      (`self.SetAbility` "NewEnumerator0")
      (`KismetSystemLibrary.K2_SetTimerDelegate` (`|CreateDelegate` :!event `BP_BallPawn_LevitateEnd`) 3.0)
      (`PrimitiveComponent.SetEnableGravity` (`self.CollisionComponent`) false)
      (`self.K2_SetActorLocation` (+ (`self.K2_GetActorLocation`) (0.0 0.0 300.0))))
    (:`NewEnumerator2`
      ;[0.2871 0.3258 0.8073 0.5] Comment
      (`self.SetAbility` "NewEnumerator0")
      (`KismetSystemLibrary.K2_SetTimerDelegate` (`|CreateDelegate` :!event `BP_BallPawn_SlowTimeEnd`) 5.0)
      (bind _outactors (`GameplayStatics.GetAllActorsOfClass` "/Game/A_Crusher.A_Crusher_C"))
      (for _array_element _outactors
        (set `Actor.CustomTimeDilation` 0.2 _array_element)))))

(fn `BP_BallPawn_LevitateEnd`
  (`PrimitiveComponent.SetEnableGravity` (`self.CollisionComponent`) true)
  (if (`|EnumEquality` (`self.CurrentAbility`) "NewEnumerator0")
    (`self.SetAbility` "NewEnumerator1")))

(fn `BP_BallPawn_SlowTimeEnd`
  (bind _outactors (`GameplayStatics.GetAllActorsOfClass` "/Game/A_Crusher.A_Crusher_C"))
  (for _array_element _outactors
    (set `Actor.CustomTimeDilation` 1.0 _array_element)
    (if (`|EnumEquality` (`self.CurrentAbility`) "NewEnumerator0")
      (`self.SetAbility` "NewEnumerator2"))))

(fn `Move`
  (params (ScaleValue :type "Float (single-precision)"))
  (`self.AddMovementInput` (`SceneComponent.GetForwardVector` (`self.MeshComponent`)) ScaleValue))

(fn `Rotate`
  (params (Amount :type "Float (double-precision)"))
  (locals (NewLocalVar :type "Rotator Structure" :default (struct)) (Rotation :type "Float (single-precision)" :default 90.0))
  (`SceneComponent.K2_AddWorldRotation` (`self.MeshComponent`) (`KismetMathLibrary.MakeRotator` 0.0 0.0 Amount) false false))

(fn `SetAbility`
  (params (NewAbility :type "/Game/E_Ability Enum" :default "NewEnumerator0"))
  (set `self.CurrentAbility` NewAbility))

(fn `UserConstructionScript`)