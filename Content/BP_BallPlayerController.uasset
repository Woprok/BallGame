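; Player controller for the ball game that routes Enhanced Input to the possessed BP_BallPawn and handles game over and restart.
; Ability, move and rotate input go to the pawn cached on possess, with axes reduced to their sign and rotation scaled by a step.
; VictoryOrLoss shows the result widget, removes ball controls and destroys the pawn.
; Restart clears widgets, restores those controls and respawns through the game mode.
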(event `EnhancedInput|/Game/Inputs/IA_Ability`
  (params (ActionValue :type Boolean) (ElapsedSeconds :type "Float (double-precision)") (TriggeredSeconds :type "Float (double-precision)") (InputAction :type "InputAction Object Reference" :default "/Game/Inputs/IA_Ability.IA_Ability"))
  (:`Triggered`
    (`/Game/BP_BallPawn.Ability` (`self.As BP Ball Pawn`))))

(event `EnhancedInput|/Game/Inputs/IA_Rotate`
  (params (ActionValue :type "Float (double-precision)") (ElapsedSeconds :type "Float (double-precision)") (TriggeredSeconds :type "Float (double-precision)") (InputAction :type "InputAction Object Reference" :default "/Game/Inputs/IA_Rotate.IA_Rotate"))
  (:`Triggered`
    (`/Game/BP_BallPawn.Rotate` (`self.As BP Ball Pawn`) (* (`KismetMathLibrary.SignOfFloat` ActionValue) (`self.RotateStep`)))))

(event `EnhancedInput|/Game/Inputs/IA_Move`
  (params (ActionValue :type "Float (double-precision)") (ElapsedSeconds :type "Float (double-precision)") (TriggeredSeconds :type "Float (double-precision)") (InputAction :type "InputAction Object Reference" :default "/Game/Inputs/IA_Move.IA_Move"))
  (:`Triggered`
    (`/Game/BP_BallPawn.Move` (`self.As BP Ball Pawn`) (`KismetMathLibrary.SignOfFloat` ActionValue))))

(event `EnhancedInput|/Game/Inputs/IA_Restart`
  (params (ActionValue :type Boolean) (ElapsedSeconds :type "Float (double-precision)") (TriggeredSeconds :type "Float (double-precision)") (InputAction :type "InputAction Object Reference" :default "/Game/Inputs/IA_Restart.IA_Restart"))
  (:`Triggered`
    (`self.Restart`)))

(event `self.ReceiveBeginPlay`
  (bind _returnvalue (subsystem `EnhancedInputLocalPlayerSubsystem`))
  (`EnhancedInputSubsystemInterface.AddMappingContext` _returnvalue "/Game/Inputs/IMC_Ball.IMC_Ball" 0 (struct))
  (`EnhancedInputSubsystemInterface.AddMappingContext` _returnvalue "/Game/Inputs/IMC_Meta.IMC_Meta" 0 (struct)))

(event `self.ReceivePossess`
  (params (PossessedPawn :type "Pawn Object Reference"))
  (bind _asbp_ball_pawn (cast `/Game/BP_BallPawn` PossessedPawn))
  (set `self.As BP Ball Pawn` _asbp_ball_pawn))

(fn `Restart`
  (`WidgetLayoutLibrary.RemoveAllWidgets`)
  (`EnhancedInputSubsystemInterface.AddMappingContext` (subsystem `EnhancedInputLocalPlayerSubsystem`) "/Game/Inputs/IMC_Ball.IMC_Ball" 0 (struct))
  (`GameModeBase.RestartPlayer` (`GameplayStatics.GetGameMode`) self))

(fn `UserConstructionScript`)

(fn `VictoryOrLoss`
  (params (IsVictory :type Boolean))
  (bind _returnvalue (`|GenericCreateObject` "/Game/WBP_GameOverScreen.WBP_GameOverScreen_C"))
  (set `self.UI` _returnvalue)
  (`UserWidget.AddToViewport` _returnvalue 0)
  (`/Game/WBP_GameOverScreen.Show` _returnvalue IsVictory)
  (`EnhancedInputSubsystemInterface.RemoveMappingContext` (subsystem `EnhancedInputLocalPlayerSubsystem`) "/Game/Inputs/IMC_Ball.IMC_Ball" (struct))
  (`self.K2_DestroyActor` (`GameplayStatics.GetPlayerPawn` 0)))